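; End-of-level trigger zone that scores the player's box placement when the VR pawn enters its box volume.
; The overlap runs CalculateRep, which checks every BP_GrabbableBox in the level and adds or subtracts one Reputation in BP_GameInstance depending on whether it is placed correctly.
; Scoring repeats on each entry, and a separate LeaveBuilding event unhides the zone actor.
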(event OnComponentBeginOverlap(Box)
  (params (OverlappedComponent :type Primitive%20Component%20Object%20Reference) (OtherActor :type Actor%20Object%20Reference) (OtherComp :type Primitive%20Component%20Object%20Reference) (OtherBodyIndex :type Integer) (bFromSweep :type Boolean) (SweepResult :type Hit%20Result%20Structure%20%28by%20ref%29))
  (Utilities|Casting|CastToVRPawn OtherActor)
  (CallFunction|CalculateRep))

(event Custom|CalculateRep
  (bind _asbp_game_instance (Utilities|Casting|CastToBP_GameInstance (Game|GetGameInstance)))
  (bind _outactors (Actor|GetAllActorsOfClass "/Game/Blueprints/BP_GrabbableBox.BP_GrabbableBox_C"))
  (for _array_element _outactors
    (if (Variables|/Game/Blueprints/BP_GrabbableBox.BP_GrabbableBox_C|GetIsPlacedCorrectly _array_element)
      (Variables|/Game/Blueprints/BP_GameInstance.BP_GameInstance_C|SetReputation _asbp_game_instance (+ (Variables|/Game/Blueprints/BP_GameInstance.BP_GameInstance_C|GetReputation _asbp_game_instance) 1))
      (else
        (Variables|/Game/Blueprints/BP_GameInstance.BP_GameInstance_C|SetReputation _asbp_game_instance (- (Variables|/Game/Blueprints/BP_GameInstance.BP_GameInstance_C|GetReputation _asbp_game_instance) 1))))))

(event EventBeginPlay)

(event Collision|EventActorBeginOverlap
  (params (OtherActor :type Actor%20Object%20Reference)))

(event EventTick
  (params (DeltaSeconds :type Float%20%28single-precision%29)))

(event EventLeaveBuilding
  (params (EndLevelZone :type 0%20End%20Level%20Zone%20Object%20Reference))
  (Rendering|SetActorHiddenInGame false))

(fn ConstructionScript)