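; Game manager that runs the timed after-hours event and hidden-room reveal leading to the boss cutscene.
; A BeginPlay timer rings a bell, sends NPCs out, then reddens lights, hides NPCs and reveals tagged items.
; That timer or secrets 1-3 open the hidden wall with recursive random-delay flickering, then trigger the cutscene after a delay.
; Secret 4 triggers it directly; a DoOnce-gated cutscene disables movement and switches view target, while final-sequence playback is unwired.
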(event Custom|AfterHours
  (Variables|Default|SetAfterHoursTriggered true)
  (Audio|PlaySound2D "/Game/Sounds/Bell.Bell" 1.0 1.0 0.0 0 0)
  (CallFunction|AllNPCsLeave)
  (Utilities|FlowControl|Delay 8.0)
  (CallFunction|MakeRoomRed)
  (CallFunction|HideRevealItems)
  (CallFunction|CanSeeHiddenDoor))

(event Custom|CanSeeHiddenDoor
  (Collision|SetCollisionEnabled (Variables|/Script/Engine.StaticMeshActor|GetStaticMeshComponent (Variables|Default|GetHiddenRoomWall)) "NoCollision")
  (Variables|Default|SetIsGlitching true)
  (CallFunction|WallGlitch)
  (Utilities|FlowControl|Delay (Variables|Default|GetCutsceneDelay))
  (CallFunction|ActivateBossCutscene))

(event Custom|WallGlitch
  (if (Variables|Default|GetIsGlitching)
    (Rendering|SetVisibility (Variables|/Script/Engine.StaticMeshActor|GetStaticMeshComponent (Variables|Default|GetHiddenRoomWall)) false false)
    (Utilities|FlowControl|Delay (Math|Random|RandomFloatinRange 0.1 0.4))
    (Rendering|SetVisibility (Variables|/Script/Engine.StaticMeshActor|GetStaticMeshComponent (Variables|Default|GetHiddenRoomWall)) true false)
    (Utilities|FlowControl|Delay (Math|Random|RandomFloatinRange 0.8 5.0))
    (CallFunction|WallGlitch)))

(event Custom|InteractedWithSecret
  (params (SecretNum :type Integer) (PlayerRef :type VR%20Pawn%20Object%20Reference))
  (switch int SecretNum
    (:1
      (Variables|Default|SetSecret1 true)
      (CallFunction|CanSeeHiddenDoor :!label _label))
    (:2
      (Variables|Default|SetSecret2 true)
      (goto _label))
    (:3
      (Variables|Default|SetSecret3 true)
      (goto _label))
    (:4
      (CallFunction|ActivateBossCutscene))))

(event Custom|ActivateBossCutscene
  (Utilities|FlowControl|DoOnce false
    (:Completed
      (Utilities|FlowControl|Delay 1e+01)
      (Pawn|Components|CharacterMovement|DisableMovement (Variables|/Script/Engine.Character|GetCharacterMovement (Game|GetPlayerCharacter 0)))
      (Game|Player|SetViewTargetwithBlend (Game|GetPlayerController (Game|GetPlayerState 0)) (Variables|Default|GetNew%20View%20Target) 0.0 "VTBlend_Linear" 0.0 false))))

(event Custom|Change%20scenes
  (Game|OpenLevel(byName) "MenuLevel1"))

(event EventBeginPlay
  (Variables|Default|SetAfterHoursTriggered false)
  (Utilities|Time|SetTimerbyEvent (delegate Custom|AfterHours) (Variables|Default|GetRedLightsDelay)))

(event Collision|EventActorBeginOverlap
  (params (OtherActor :type Actor%20Object%20Reference)))

(event EventTick
  (params (DeltaSeconds :type Float%20%28single-precision%29)))

(fn ConstructionScript)

(fn MakeRoomRed
  (bind _outactors (Actor|GetAllActorsOfClass "/Game/Blueprints/BP_CeilingLight.BP_CeilingLight_C"))
  (for _array_element _outactors
    (Default|TurnLightsRed _array_element)
    (Class|BPIAudioControl|SwapAudio(Message) (Variables|Default|GetAudio))))

(fn HideRevealItems
  (bind _outactors (Actor|GetAllActorswithTag (Variables|Default|GetNPCTag)))
  (for _array_element _outactors
    (Rendering|SetActorHiddenInGame _array_element true)
    (Collision|SetActorEnableCollision _array_element false))
  (bind _outactors_2 (Actor|GetAllActorswithTag (Variables|Default|GetHiddenItemsTag)))
  (for _array_element_2 _outactors_2
    (Rendering|SetActorHiddenInGame _array_element_2 false)
    (Collision|SetActorEnableCollision _array_element_2 true)))

(fn AllNPCsLeave
  (bind _outactors (Actor|GetAllActorswithTag (Variables|Default|GetNPCTag)))
  (for _array_element _outactors
    (Class|BPINPCLeave|LeaveBuilding(Message) _array_element (Variables|Default|GetEndLevelZone))))