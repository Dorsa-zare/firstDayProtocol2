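; BP_NPCManager populates the level with a random crowd of male and female NPCs when play begins.
; On BeginPlay it gathers every BP_Spawner in the level and loops a random number of times bounded by MinSpawned and MaxSpawned.
; Each pass picks man or woman at even odds, spawns it at a randomly chosen spawner's transform, and stores only the latest of each in NPCMale or NPCFem.
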(event EventBeginPlay
  (bind _outactors (Actor|GetAllActorsOfClass "/Game/Blueprints/BP_Spawner.BP_Spawner_C"))
  (for _index (range 0 (Math|Random|RandomIntegerinRange (Variables|Default|GetMinSpawned) (Variables|Default|GetMaxSpawned)))
    (if (== (Math|Random|RandomIntegerinRange 0 1) 0)
      (bind _returnvalue (Game|SpawnActorfromClass "/Game/Characters/NPC_Man.NPC_Man_C" (Transformation|GetActorTransform (Utilities|Array|Get(acopy) _outactors (Math|Random|RandomIntegerinRange 0 (- (Utilities|Array|Length _outactors) 1)))) "Undefined" "MultiplyWithRoot" 0 0))
      (Variables|Default|SetNPCMale _returnvalue)
      (else
        (bind _returnvalue_2 (Game|SpawnActorfromClass "/Game/Characters/NPC_Woman.NPC_Woman_C" (Transformation|GetActorTransform (Utilities|Array|Get(acopy) _outactors (Math|Random|RandomIntegerinRange 0 (- (Utilities|Array|Length _outactors) 1)))) "Undefined" "MultiplyWithRoot" 0 0))
        (Variables|Default|SetNPCFem _returnvalue_2)))))

(event EventTick
  (params (DeltaSeconds :type Float%20%28single-precision%29)))

(fn ConstructionScript)