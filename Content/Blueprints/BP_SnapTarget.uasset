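; BP_SnapTarget is a snap point for BP_GrabbableBox actors that records whether the correct box was placed.
; TargetArea overlap tracks the interacting box and registers this target as its CurrentSnapPoint.
; CheckBox snaps an unheld box into a free target, disabling physics, moving it to TargetArea and marking the target occupied.
; SnapBox then compares it with CorrectBox, sets IsPlacedCorrectly and fires OnBoxSnapped.
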(event OnComponentBeginOverlap(TargetArea)
  (params (OverlappedComponent :type Primitive%20Component%20Object%20Reference) (OtherActor :type Actor%20Object%20Reference) (OtherComp :type Primitive%20Component%20Object%20Reference) (OtherBodyIndex :type Integer) (bFromSweep :type Boolean) (SweepResult :type Hit%20Result%20Structure%20%28by%20ref%29))
  (if (not (Variables|Default|GetIsOccupied))
    (bind _asbp_grabbable_box (Utilities|Casting|CastToBP_GrabbableBox OtherActor))
    (bind _output_get (Variables|Default|SetInteractingBox _asbp_grabbable_box))
    (Variables|Default|SetbCanSnap true)
    (Variables|/Game/Blueprints/BP_GrabbableBox.BP_GrabbableBox_C|SetCurrentSnapPoint _output_get self)
    (CallFunction|CheckBox _output_get)))

(event OnComponentEndOverlap(TargetArea)
  (params (OverlappedComponent :type Primitive%20Component%20Object%20Reference) (OtherActor :type Actor%20Object%20Reference) (OtherComp :type Primitive%20Component%20Object%20Reference) (OtherBodyIndex :type Integer))
  (if (== OtherActor (Variables|Default|GetInteractingBox))
    (Variables|Default|SetbCanSnap false)
    (Variables|Default|SetInteractingBox 0)))

(event Custom|SnapBox
  (params (BoxRef :type BP%20Grabbable%20Box%20Object%20Reference))
  (bind _interactingbox (Variables|Default|GetInteractingBox))
  (Variables|Default|SetbGrabComponent (Variables|/Game/Blueprints/BP_GrabbableBox.BP_GrabbableBox_C|GetGrabComponent BoxRef))
  (if (and (Utilities|IsValid BoxRef) (not (Variables|/Game/VRTemplate/Blueprints/GrabComponent.GrabComponent_C|GetbIsHeld (Variables|Default|GetbGrabComponent))))
    (Physics|SetSimulatePhysics (Variables|/Game/Blueprints/BP_GrabbableBox.BP_GrabbableBox_C|GetStaticMesh BoxRef) false)
    (Transformation|SetActorLocationAndRotation (Variables|Default|GetInteractingBox) (Transformation|GetWorldLocation (Variables|Default|GetTargetArea)))
    (Variables|/Game/VRTemplate/Blueprints/GrabComponent.GrabComponent_C|SetIsSnapped (Variables|Default|GetbGrabComponent) true)
    (Variables|Default|SetIsOccupied true)
    (if (== _interactingbox (Variables|Default|GetCorrectBox))
      (Variables|/Game/Blueprints/BP_GrabbableBox.BP_GrabbableBox_C|SetIsPlacedCorrectly _interactingbox true)
      (else
        (Variables|/Game/Blueprints/BP_GrabbableBox.BP_GrabbableBox_C|SetIsPlacedCorrectly _interactingbox false)))
    (Default|CallOnBoxSnapped (Variables|Default|GetInteractingBox))))

(event Custom|CheckBox
  (params (Grabbed%20Box :type BP%20Grabbable%20Box%20Object%20Reference))
  (if (Math|Boolean|ANDBoolean (not (Variables|/Game/VRTemplate/Blueprints/GrabComponent.GrabComponent_C|GetbIsHeld (Variables|/Game/Blueprints/BP_GrabbableBox.BP_GrabbableBox_C|GetGrabComponent Grabbed%20Box))) (Variables|Default|GetbCanSnap) (not (Variables|Default|GetIsOccupied)))
    (CallFunction|SnapBox Grabbed%20Box)))

(event EventBeginPlay)

(event Collision|EventActorBeginOverlap
  (params (OtherActor :type Actor%20Object%20Reference)))

(fn ConstructionScript)